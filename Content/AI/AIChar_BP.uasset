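; AI enemy character Blueprint that takes damage, respawns and fires projectiles.
; Any damage reduces Health; at zero it teleports far below the level, then after a short delay restores health and moves to a random SpawnPoint gathered on BeginPlay.
; StartShooting and StopShooting toggle a looping timer that spawns AIProj_BP from the Arrow1 transform at FireRate.
; A HealthBonus event sets Health to a passed-in maximum.
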(event `self.ReceiveBeginPlay`
  ;[1 1 1] AI Respawn
  (bind _outactors (`GameplayStatics.GetAllActorsOfClass` "/Game/Spawner/SpawnPoint.SpawnPoint_C"))
  (set `self.SpawnPoint` _outactors))

(event `Respawn`
  (bind _spawnpoint (`self.SpawnPoint`))
  ;[1 1 1] AI Respawn
  (`KismetSystemLibrary.Delay` 2.0)
  (set `self.Health` 100.0)
  (`self.K2_SetActorLocation` (`self.K2_GetActorLocation` (`|GetArrayItem` _spawnpoint (`KismetMathLibrary.RandomIntegerInRange` 0 (- (`KismetArrayLibrary.Array_Length` _spawnpoint) 1)))) false true))

(event `self.ReceiveAnyDamage`
  (params (Damage :type "Float (single-precision)") (DamageType :type "DamageType Object Reference") (InstigatedBy :type "Controller Object Reference") (DamageCauser :type "Actor Object Reference"))
  ;[1 1 1] Health and Damage
  ;;[1 1 1] Checks to see if there is damage being applied
  (set `self.Damage Causer` DamageCauser)
  (set `self.Health` (- (`self.Health`) Damage))
  (`self.CheckHealth`)
  (`KismetSystemLibrary.PrintString` (`KismetStringLibrary.Conv_DoubleToString` (`self.Health`)) true true (struct :`R` 1.0 :`B` 0.004046 :`A` 1.0)))

(event `CheckHealth`
  ;[1 1 1] Health and Damage
  ;;[1 1 1] Checks Player Health
  (if (<= (`self.Health`) 0.0)
    (`self.K2_SetActorLocation` (0.0 0.0 -5000.0) false true)
    (`self.Respawn`)))

(event `HealthBonus`
  (params (MaxHealth :type "Float (double-precision)"))
  ;[1 1 1] Health and Damage
  ;;[1 1 1] Adds health to health
  (bind _output_get (set `self.MaxHealth` MaxHealth))
  (set `self.Health` _output_get))

(event `StartShooting`
  ;[1 1 1] AI Starts shooting
  (`KismetSystemLibrary.K2_SetTimer` null "AIShoot" (`self.FireRate`) true))

(event `StopShooting`
  ;[1 1 1] Tells AI to stop shooting
  (`KismetSystemLibrary.K2_ClearTimer` null "AIShoot"))

(event `AIShoot`
  ;[1 1 1] Makes AI projectile spawn from enemy pawn
  (`|SpawnActorFromClass` "/Game/AI/AIProj_BP.AIProj_BP_C" (`SceneComponent.K2_GetComponentToWorld` (`self.Arrow1`)) "Undefined" "MultiplyWithRoot" self null))

(fn `UserConstructionScript`)