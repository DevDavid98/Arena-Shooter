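; Player character Blueprint for a shooter, with camera-relative movement, jumping, an AK-47-style automatic weapon and a HUD widget.
; Holding Shoot loops a timer that traces from the camera, then spawns projectiles from the muzzle arrow toward the aim point.
; Ammo limits firing, and a delayed reload refills it only once depleted below zero.
; Damage reduces health, with death restoring it and teleporting the player to a random SpawnPoint.
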(event `self.ReceiveBeginPlay`
  (bind _outactors (`GameplayStatics.GetAllActorsOfClass` "/Game/Spawner/SpawnPoint.SpawnPoint_C"))
  (set `self.SpawnPoint` _outactors)
  (bind _returnvalue (`|CreateWidget` "/Game/UI/player_W.player_W_C"))
  (bind _output_get (set `self.player_W` _returnvalue))
  (`UserWidget.AddToViewport` _output_get 0))

(event `Respawn`
  (bind _spawnpoint (`self.SpawnPoint`))
  (set `self.Health` 100.0)
  (`self.K2_SetActorLocation` (`self.K2_GetActorLocation` (`|GetArrayItem` _spawnpoint (`KismetMathLibrary.RandomIntegerInRange` 0 (- (`KismetArrayLibrary.Array_Length` _spawnpoint) 1)))) false true))

(event `InputAxis|MoveForword`
  (params (AxisValue :type "Float (single-precision)"))
  (bind (_returnvalue_roll _returnvalue_pitch _returnvalue_yaw) (`KismetMathLibrary.BreakRotator` (`self.GetControlRotation`)))
  ;[1 1 1] Move forward backword, left and right
  (`self.AddMovementInput` (`KismetMathLibrary.GetForwardVector` (`KismetMathLibrary.MakeRotator` 0.0 0.0 _returnvalue_yaw)) AxisValue))

(event `InputAxis|MoveRight`
  (params (AxisValue :type "Float (single-precision)"))
  (bind (_returnvalue_roll _returnvalue_pitch _returnvalue_yaw) (`KismetMathLibrary.BreakRotator` (`self.GetControlRotation`)))
  ;[1 1 1] Move forward backword, left and right
  (`self.AddMovementInput` (`KismetMathLibrary.GetRightVector` (`KismetMathLibrary.MakeRotator` 0.0 0.0 _returnvalue_yaw)) AxisValue))

(event `InputAxis|Turn`
  (params (AxisValue :type "Float (single-precision)"))
  ;[1 1 1] Look up,down, left and right
  (`self.AddControllerYawInput` AxisValue))

(event `InputAction|Jump`
  (params (Key :type "Key Structure"))
  ;[1 1 1] Player Jump
  (:`Pressed`
    (`self.Jump`))
  (:`Released`
    (`self.StopJumping`)))

(event `InputAxis|LookUp`
  (params (AxisValue :type "Float (single-precision)"))
  ;[1 1 1] Look up,down, left and right
  (`self.AddControllerPitchInput` AxisValue))

(event `self.ReceiveAnyDamage`
  (params (Damage :type "Float (single-precision)") (DamageType :type "DamageType Object Reference") (InstigatedBy :type "Controller Object Reference") (DamageCauser :type "Actor Object Reference"))
  ;[1 1 1] Health and Damage
  ;;[1 1 1] Checks to see if there is damage being applied
  (set `self.Damage Causer` DamageCauser)
  (set `self.Health` (- (`self.Health`) Damage))
  (`self.CheckHP`)
  (`KismetSystemLibrary.PrintString` (`KismetStringLibrary.Conv_DoubleToString` (`self.Health`)) true true (struct :`G` 1.0 :`B` 0.12776 :`A` 1.0)))

(event `CheckHP`
  ;[1 1 1] Health and Damage
  ;;[1 1 1] Checks Player Health
  (if (<= (`self.Health`) 0.0)
    (`self.Respawn`)))

(event `HealthBonus`
  (params (MaxHealth :type "Float (double-precision)"))
  ;[1 1 1] Health and Damage
  ;;[1 1 1] Adds health to health
  (bind _output_get (set `self.MaxHealth` MaxHealth))
  (set `self.Health` _output_get))

(event `AutoFire`
  ;[1 1 1] Shooting Logic
  (`self.LineTraceAutoFire`))

(event `InputAction|Shoot`
  (params (Key :type "Key Structure"))
  ;[1 1 1] Shooting Logic
  (:`Pressed`
    (`KismetSystemLibrary.K2_SetTimer` null "Autofire" (`self.fireRate`) true))
  (:`Released`
    (`KismetSystemLibrary.K2_ClearTimer` null "Autofire")))

(event `InputAction|Reload`
  (params (Key :type "Key Structure"))
  ;[1 1 1] Shooting Logic
  (:`Pressed`
    (if true
      (if (< (`self.AmmoCount`) 0)
        (set `self.Can Realod` (`self.no reload`))
        (`GameplayStatics.PlaySoundAtLocation` "/Game/FPWeapon/Audio/ak47_reload.ak47_reload" (`SceneComponent.K2_GetComponentLocation` (`self.akm_47`)) (struct) 1.0 1.0 0.0 null null null null)
        (`KismetSystemLibrary.Delay` 2.2)
        (set `self.AmmoCount` (`self.Max Ammo`))
        (set `self.Can Realod` true)
        (else
          (set `self.Can Realod` (`self.no reload`)))))))

(fn `CheckHealth`)

(fn `LineTraceAutoFire`
  (bind _returnvalue (`GameplayStatics.GetPlayerCameraManager` 0))
  (bind _returnvalue_2 (`PlayerCameraManager.GetCameraLocation` _returnvalue))
  (bind _returnvalue_3 (`SceneComponent.K2_GetComponentLocation` (`self.Arrow1`)))
  (if (>= (`self.AmmoCount`) 0)
    (bind _outhit (`KismetSystemLibrary.LineTraceSingle` :`Start` _returnvalue_2 :`End` (+ _returnvalue_2 (* (`KismetMathLibrary.GetForwardVector` (`PlayerCameraManager.GetCameraRotation` _returnvalue)) 50000.0)) :`TraceChannel` "TraceTypeQuery1" :`DrawDebugType` "ForDuration"))
    (`|SpawnActorFromClass` "/Game/Player/PlayerProj_BP.PlayerProj_BP_C" (`KismetMathLibrary.MakeTransform` _returnvalue_3 (`KismetMathLibrary.MakeRotFromX` (`KismetMathLibrary.Normal` (- (`KismetMathLibrary.SelectVector` (`.Location` (`GameplayStatics.BreakHitResult` _outhit)) (`.TraceEnd` (`GameplayStatics.BreakHitResult` _outhit)) (`GameplayStatics.BreakHitResult` _outhit)) _returnvalue_3)))) "Undefined" "MultiplyWithRoot" null null)
    (`GameplayStatics.PlaySoundAtLocation` "/Game/FPWeapon/Audio/ak47_shoot.ak47_shoot" (`SceneComponent.K2_GetComponentLocation` (`self.Arrow1`)) (struct) 1.0 1.0 0.0 null null null null)
    (set `self.AmmoCount` (- (`self.AmmoCount`) 1))
    (else
      (`KismetSystemLibrary.K2_ClearTimer` null "Autofire"))))

(fn `UserConstructionScript`)